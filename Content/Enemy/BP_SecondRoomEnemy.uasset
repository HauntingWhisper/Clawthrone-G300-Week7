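; BP_SecondRoomEnemy is an AI enemy that patrols waypoints and moves toward noises it hears.
; BeginPlay starts a looping AIMoveTo patrol with pauses; PawnSensing hearing issues a move to the noise and plays a sound at world origin.
; Tick updates a camera-facing health bar widget from the health component, whose depletion destroys the actor.
; Sight handling is empty, and the random-roam loop is never called.
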(event OnHealthChanged(BP_HealthComponent)
  (params (NewHealth :type Float%20%28double-precision%29)))

(event OnHealthDepleted(BP_HealthComponent)
  (Actor|DestroyActor))

(event OnSeePawn(PawnSensing)
  (params (Pawn :type Pawn%20Object%20Reference)))

(event OnHearNoise(PawnSensing)
  (params (Instigator :type Pawn%20Object%20Reference) (Location :type Vector%20%28by%20ref%29 :default "0, 0, 0") (Volume :type Float%20%28single-precision%29))
  (AI|AIMoveTo self Location 0 5.0 false
    (:then
      (Audio|PlaySoundatLocation "/Game/LevelPrototyping/Sounds/Nani.Nani" "0, 0, 0" "0, 0, 0" 1.0 1.0 0.0 0 0 0 0))))

(event Custom|MoveRandom
  (AI|AIMoveTo self (.RandomLocation (AI|Navigation|GetRandomReachablePointinRadius (Transformation|GetActorLocation) 3e+03 0 0)) 0 5.0 false :!label _label
    (:OnSuccess
      (Utilities|FlowControl|Delay 1.0)
      (goto _label))))

(event Custom|BeginPatrol
  (bind _waypoints (Variables|Default|GetWaypoints))
  (AI|AIMoveTo self "0, 0, 0" (Utilities|Array|Get(acopy) _waypoints (Variables|Default|GetCurrentWaypoint)) 5.0 false :!label _label
    (:OnSuccess
      (Math|Integer|IncrementInt (Variables|Default|GetCurrentWaypoint)
        (:%20%20
          (if (>= (Variables|Default|GetCurrentWaypoint) (Utilities|Array|Length _waypoints))
            (Variables|Default|SetCurrentWaypoint 0))
          (Utilities|FlowControl|Delay 5.0)
          (goto _label))))))

(event EventBeginPlay
  (CallFunction|BeginPatrol))

(event Collision|EventActorBeginOverlap
  (params (OtherActor :type Actor%20Object%20Reference)))

(event EventTick
  (params (DeltaSeconds :type Float%20%28single-precision%29))
  (bind _bp_healthcomponent (Variables|Default|GetBP_HealthComponent))
  (bind _healthwidget (Variables|Default|GetHealthWidget))
  (bind _asbp_health_bar (Utilities|Casting|CastToBP_HealthBar (UserInterface|GetWidget (Variables|Default|GetHealthWidget))))
  (Progress|SetPercent (Variables|/Game/Components/BP_HealthBar.BP_HealthBar_C|GetHealthBarElement _asbp_health_bar) (/ (Variables|/Game/Components/BP_HealthComponent.BP_HealthComponent_C|GetHealth _bp_healthcomponent) (Variables|/Game/Components/BP_HealthComponent.BP_HealthComponent_C|GetMax%20Health _bp_healthcomponent)))
  (Transformation|SetWorldRotation _healthwidget (Math|Rotator|FindLookatRotation (Transformation|GetWorldLocation _healthwidget) (Transformation|GetWorldLocation (Variables|/Script/Engine.PlayerCameraManager|GetTransformComponent (Game|GetPlayerCameraManager 0)))) false false))

(fn ConstructionScript)